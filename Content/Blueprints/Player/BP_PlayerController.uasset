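; Player controller that opens the character menu and handles respawning of the player character.
; Pressing Tab creates and shows Widget_Character, pauses the game and shows the mouse cursor.
; The Respawn event spawns a new BP_Character at the game mode's player start, adjusting for collisions, and possesses it.
; A similar chain for opening an inventory widget is present but disconnected, so it never runs.
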(event `Key|Tab`
  (params (Key :type "Key Structure"))
  (:`Pressed`
    (bind _returnvalue (`|CreateWidget` "/Game/UI/Widget_Character.Widget_Character_C" self))
    (`UserWidget.AddToViewport` _returnvalue 0)
    (`GameplayStatics.SetGamePaused` true)
    (set `self.bShowMouseCursor` true)))

(event `InputAction|Inventory`
  (params (Key :type "Key Structure")))

(event `Respawn`
  (bind _returnvalue (`|SpawnActorFromClass` "/Game/Blueprints/Player/BP_Character.BP_Character_C" (`self.GetTransform` (`GameModeBase.K2_FindPlayerStart` (`GameplayStatics.GetGameMode`) self "")) "AdjustIfPossibleButAlwaysSpawn" "OverrideRootScale" null null))
  (`self.Possess` _returnvalue))

(fn `UserConstructionScript`)