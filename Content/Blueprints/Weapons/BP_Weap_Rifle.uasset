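; Rifle weapon Blueprint that fires instant-hit shots automatically while firing is active.
; BeginPlay clamps Ammo to MaxAmmo and fills the magazine from it, capped at MaxMagAmmo.
; StartFire runs Fire on a looping FireRate timer, so the first shot waits one interval, and StopFire clears that timer.
; Each Fire calls the hit, fire-simulation and ammo-use functions, which are defined outside these graphs.
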(event `self.ReceiveBeginPlay`
  (`parent.ReceiveBeginPlay`)
  (set `self.Ammo` (`KismetMathLibrary.Min` (`self.Ammo`) (`self.MaxAmmo`)))
  (set `self.MagAmmo` (`KismetMathLibrary.Min` (`self.MaxMagAmmo`) (`self.Ammo`))))

(event `self.Fire`
  (`self.FireInstantHit`)
  (`self.SimulateWeaponFire`)
  (`self.UseAmmo`))

(event `self.StartFire`
  (bind _returnvalue (`KismetSystemLibrary.K2_SetTimer` null "Fire" (`self.FireRate`) true))
  (set `self.FiringHandle` _returnvalue))

(event `self.StopFire`
  (`KismetSystemLibrary.K2_ClearAndInvalidateTimerHandle` (`self.FiringHandle`)))

(fn `UserConstructionScript`
  (`parent.UserConstructionScript`))