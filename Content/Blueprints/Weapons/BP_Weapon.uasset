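; BP_Weapon is a first-person weapon actor that attaches to the owning pawn's hands and manages firing state and ammo.
; StartFire calls Fire, which plays the montage and sound and decrements ammo, then changes the weapon state.
; Separate hitscan (camera trace, headshot multiplier, impulse) and projectile functions exist, but Fire calls neither.
; CanFire is likewise uncalled here, and Reload only computes a delta without refilling the magazine.
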(event `self.ReceiveBeginPlay`
  (`self.SetWeaponState` "NewEnumerator0"))

(event `Fire`
  (`self.SimulateWeaponFire`)
  (`self.UseAmmo`))

(event `StartFire`
  (`self.Fire`)
  (`self.SetWeaponState` "NewEnumerator1"))

(event `StopFire`
  (`self.SetWeaponState` "NewEnumerator0"))

(fn `AddAmmo`
  (params (AmmoAmount :type Integer))
  (returns (Ammo :type Integer))
  (locals (AmmoDelta :type Integer))
  (bind _output_get (set `local.AmmoDelta` (`KismetMathLibrary.Max` (- (`self.MaxAmmo`) (`self.Ammo`)))))
  (set `self.Ammo` (+ (`KismetMathLibrary.Min` _output_get AmmoAmount) 1))
  (return (`KismetMathLibrary.Max` 0 (- AmmoAmount (`local.AmmoDelta`)))))

(fn `AttachToOwner`
  (`SceneComponent.K2_AttachToComponent` (`self.WeaponMesh`) (`/Game/Blueprints/Player/BP_Character.FirstPersonMesh` (`self.PawnOwner`)) (`self.HandsAttachSocket`) "SnapToTarget" "SnapToTarget" "SnapToTarget" true))

(fn `CanFire`
  (returns (CanFire :type Boolean))
  (return (or (== (`self.WeaponState`) (enumliteral `/Game/Blueprints/Weapons/EWeaponState` "NewEnumerator0")) (== (`self.WeaponState`) (enumliteral `/Game/Blueprints/Weapons/EWeaponState` "NewEnumerator1")))))

(fn `DetachFromOwner`
  (`SceneComponent.K2_DetachFromComponent` (`self.WeaponMesh`) "KeepRelative" "KeepRelative" "KeepRelative" true))

(fn `FireInstantHit`
  (bind _charactercameracomponent (`/Game/Blueprints/Player/BP_Character.CharacterCameraComponent` (`self.PawnOwner`)))
  (bind _returnvalue (`SceneComponent.K2_GetComponentLocation` _charactercameracomponent))
  (bind (_outhit _returnvalue_2) (`KismetSystemLibrary.LineTraceSingle` _returnvalue (+ _returnvalue (* (`KismetMathLibrary.GetForwardVector` (`SceneComponent.K2_GetComponentRotation` _charactercameracomponent)) (`self.MaxTraceDist`))) "TraceTypeQuery3" true (`|MakeArray` self (`self.PawnOwner`) :!type "Actor Object Reference") "ForDuration"))
  (if _returnvalue_2
    (bind (_bblockinghit _binitialoverlap _time _distance _location _impactpoint _normal _impactnormal _physmat _hitactor _hitcomponent _hitbonename) (`GameplayStatics.BreakHitResult` _outhit))
    (if (== _hitbonename "head")
      ;[0 0 0] Replace with physical material headshot damage
      (`GameplayStatics.ApplyDamage` _hitactor (* (`self.HeadshotMultiplier`) (`self.Damage`)) (`GameplayStatics.GetPlayerController` 0) self)
      (`/Engine/EditorBlueprintResources/StandardMacros.IsValid` _hitcomponent
        (:`Is Valid`
          (`PrimitiveComponent.AddImpulseAtLocation` _hitcomponent (* _location (`self.ImpulseVelcoity`)) (0.0 0.0 0.0) "None")))
      (else
        (`GameplayStatics.ApplyDamage` _hitactor (`self.Damage`) (`GameplayStatics.GetPlayerController` 0) self)
        (`/Engine/EditorBlueprintResources/StandardMacros.IsValid` _hitcomponent
          (:`Is Valid`
            (`PrimitiveComponent.AddImpulseAtLocation` _hitcomponent (* _location (`self.ImpulseVelcoity`)) _location _hitbonename)))))))

(fn `FireProjectile`
  (bind _weaponmesh (`self.WeaponMesh`))
  (`|SpawnActorFromClass` (`self.ProjectileClass`) (`SceneComponent.GetSocketTransform` _weaponmesh (`SkinnedMeshComponent.GetSocketBoneName` _weaponmesh (`self.MuzzeLocation`)) "RTS_World") "AlwaysSpawn" "OverrideRootScale" self (`self.PawnOwner`)))

(fn `Reload`
  (locals (MagDelta :type Integer))
  (bind _output_get (set `local.MagDelta` (`KismetMathLibrary.Min` (- (`self.MaxMagAmmo`) (`self.MagAmmo`)) (- (`self.Ammo`) (`self.MagAmmo`)))))
  (if (> _output_get 0)
    (set `local.MagDelta` (+ (`self.MagAmmo`) 1))))

(fn `SetWeaponOwner`
  (params (NewOwner :type "/Game/Blueprints/Player/BP_Character Object Reference"))
  (`/Engine/EditorBlueprintResources/StandardMacros.IsValid` NewOwner
    (:`Is Valid`
      (`self.SetOwner` NewOwner NewOwner)
      (set `self.Instigator` NewOwner)
      (set `self.PawnOwner` NewOwner))))

(fn `SetWeaponState`
  (params (NewState :type "/Game/Blueprints/Weapons/EWeaponState Enum" :default "NewEnumerator0"))
  (set `self.WeaponState` NewState))

(fn `SimulateWeaponFire`
  (`AnimInstance.Montage_Play` (`SkeletalMeshComponent.GetAnimInstance` (`/Game/Blueprints/Player/BP_Character.FirstPersonMesh` (`self.PawnOwner`))) "/Game/FirstPerson/Animations/FirstPersonFire_Montage.FirstPersonFire_Montage" 1.0 "MontageLength" 0.0 true)
  (`GameplayStatics.SpawnSoundAttached` (`self.FireSound`) (`self.WeaponMesh`) "None" (0.0 0.0 0.0) (struct) "KeepRelativeOffset" false 1.0 1.0 0.0 null null))

(fn `UseAmmo`
  (bind _result (`/Engine/EditorBlueprintResources/StandardMacros.DecrementInt` (`self.MagAmmo`))
    (:`  `
      (set `self.MagAmmo` _result)
      (bind _result_2 (`/Engine/EditorBlueprintResources/StandardMacros.DecrementInt` (`self.Ammo`))
        (:`  `
          (set `self.Ammo` _result_2))))))

(fn `UserConstructionScript`
  (`parent.UserConstructionScript`))