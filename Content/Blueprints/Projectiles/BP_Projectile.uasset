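; Projectile actor that deals damage on hit and limits its lifetime to a few seconds from BeginPlay.
; A valid hit applies point damage if the collision sphere's radius is zero or less, otherwise radial damage at the impact point using DamageParams.OuterRadius.
; Damage is always credited to player controller 0, and the hit handler does not destroy the projectile.
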(event `self.ReceiveBeginPlay`
  (`self.SetLifeSpan` 5.0))

(event `self.SphereCollisionComp.OnComponentHit`
  (params (HitComponent :type "PrimitiveComponent Object Reference") (OtherActor :type "Actor Object Reference") (OtherComp :type "PrimitiveComponent Object Reference") (NormalImpulse :type "Vector Structure") (Hit :type "HitResult Structure (by ref)"))
  (bind (_bblockinghit _binitialoverlap _time _distance _location) (`GameplayStatics.BreakHitResult` Hit))
  (bind _returnvalue (`GameplayStatics.GetPlayerController` 0))
  (bind (_damageparams_basedamage _damageparams_minimumdamage _damageparams_innerradius _damageparams_outerradius) (break `RadialDamageParams` (`self.DamageParams`)))
  (`/Engine/EditorBlueprintResources/StandardMacros.IsValid` OtherActor
    (:`Is Valid`
      (if (<= (`SphereComponent.SphereRadius` (`self.SphereCollisionComp`)) 0.0)
        (`GameplayStatics.ApplyPointDamage` null _damageparams_basedamage _location Hit _returnvalue self)
        (else
          (`GameplayStatics.ApplyRadialDamage` _damageparams_basedamage _location _damageparams_outerradius null (`|MakeArray` self :!type "Actor Object Reference") null _returnvalue false "ECC_Camera"))))))

(fn `UserConstructionScript`)