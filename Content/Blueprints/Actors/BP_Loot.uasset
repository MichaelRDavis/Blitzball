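; BP_Loot is a damageable actor that spawns loot and destroys itself.
; On AnyDamage, it acts when positive damage is less than or equal to Health, which is never decremented, so larger hits do nothing.
; SpawnLoot spawns every class in the Pickups and PickupItems arrays at the actor's transform, adjusting for collisions but always spawning.
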(event `self.ReceiveAnyDamage`
  (params (Damage :type "Float (single-precision)") (DamageType :type "DamageType Object Reference") (InstigatedBy :type "Controller Object Reference") (DamageCauser :type "Actor Object Reference"))
  (if (> Damage 0.0)
    (if (<= (- Damage (`self.Health`)) 0.0)
      (`self.SpawnLoot`)
      (`self.K2_DestroyActor`))))

(fn `SpawnLoot`
  (bind _returnvalue (`self.GetTransform`))
  (`|ExecutionSequence`
    (:`then_0`
      (for _array_element (`self.Pickups`)
        (`|SpawnActorFromClass` _array_element _returnvalue "AdjustIfPossibleButAlwaysSpawn" "OverrideRootScale" null null)))
    (:`then_1`
      (for _array_element_2 (`self.PickupItems`)
        (`|SpawnActorFromClass` _array_element_2 _returnvalue "AdjustIfPossibleButAlwaysSpawn" "OverrideRootScale" null null)))))

(fn `UserConstructionScript`)