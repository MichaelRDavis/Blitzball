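; BP_Destructable is a damageable actor that spawns a pickup when it is destroyed.
; Any positive damage sets Health to Damage minus Health (operands reversed from a usual decrement), and the actor destroys itself when the result is zero or less.
; Its Destroyed event spawns the Pickup class at the actor's transform, adjusting for collision but always spawning.
; Both destruction and item spawn write Visual Logger text entries.
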(event `self.ReceiveAnyDamage`
  (params (Damage :type "Float (single-precision)") (DamageType :type "DamageType Object Reference") (InstigatedBy :type "Controller Object Reference") (DamageCauser :type "Actor Object Reference"))
  (if (> Damage 0.0)
    (bind _output_get (set `self.Health` (- Damage (`self.Health`))))
    (if (<= _output_get 0.0)
      (`self.K2_DestroyActor`)
      (`VisualLoggerKismetLibrary.LogText` null "Destroyed" "VisLogBP_Destructable" true))))

(event `self.ReceiveDestroyed`
  (`|SpawnActorFromClass` (`self.Pickup`) (`self.GetTransform`) "AdjustIfPossibleButAlwaysSpawn" "OverrideRootScale" null null)
  (`VisualLoggerKismetLibrary.LogText` null "Item spawned" "VisLogBP_Destructable" true))

(fn `UserConstructionScript`)