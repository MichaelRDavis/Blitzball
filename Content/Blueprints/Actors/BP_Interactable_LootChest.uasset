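; Loot chest interactable that spawns a random weapon loot actor whenever a character uses it.
; OnUsed picks a class from the WeapLoot array with a hard-coded index range and spawns it slightly offset from the chest, with the user as Instigator.
; The DestroyActor node is unconnected, so the chest does not destroy itself after use.
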(event `self.ReceiveBeginPlay`
  (`parent.ReceiveBeginPlay`))

(event `self.OnUsed`
  (params (Character :type "/Game/Blueprints/Player/BP_Character Object Reference"))
  (bind _returnvalue_location (`KismetMathLibrary.BreakTransform` (`self.GetTransform`)))
  (`|SpawnActorFromClass` (`|GetArrayItem` (`self.WeapLoot`) (`KismetMathLibrary.RandomInteger` 10)) (`KismetMathLibrary.MakeTransform` (+ _returnvalue_location (0.0 20.0 0.0))) "AdjustIfPossibleButAlwaysSpawn" "OverrideRootScale" null Character))

(fn `UserConstructionScript`
  (`parent.UserConstructionScript`))