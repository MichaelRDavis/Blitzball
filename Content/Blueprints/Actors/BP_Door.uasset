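; BP_Door is a usable door actor that swings its DoorMesh open when used.
; OnUsed checks IsOpen, then plays Timeline_0 from a closed state or reverses it from an open one.
; Timeline updates set a fixed open rotation rather than an interpolated one and flag the door open.
; The Finished output snaps the mesh back to zero rotation and clears IsOpen.
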(event `self.ReceiveBeginPlay`
  (`parent.ReceiveBeginPlay`))

(event `self.OnUsed`
  (params (Character :type "/Game/Blueprints/Player/BP_Character Object Reference"))
  (if (not (`self.IsOpen`))
    (`Timeline|Timeline_0` :!label _label
      (:`Update`
        (`SceneComponent.K2_SetRelativeRotation` (`self.DoorMesh`) (struct :`Yaw` -145.0) false false)
        (set `self.IsOpen` true))
      (:`Finished`
        (`SceneComponent.K2_SetRelativeRotation` :`self` (`self.DoorMesh`))
        (set `self.IsOpen` false)))
    (else
      (goto _label :!via `Reverse`))))

(fn `UserConstructionScript`
  (`parent.UserConstructionScript`))