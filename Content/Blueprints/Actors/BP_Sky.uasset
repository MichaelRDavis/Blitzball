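; BP_Sky is a sky actor that drives a day-night cycle from a rotating directional light.
; Each tick it pitches the light by SunSpeed, updates the sun direction, and flags night when the light's pitch is within the threshold range.
; Only when that flag changes, Night or Day switches light intensity plus sun and star brightness, then the sky material refreshes.
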(event `self.ReceiveTick`
  (params (DeltaSeconds :type "Float (single-precision)"))
  (bind _directional_light_actor (`self.Directional light actor`))
  (bind _isnight (`self.IsNight`))
  (`self.K2_AddActorLocalRotation` _directional_light_actor (`KismetMathLibrary.MakeRotator` 0.0 (* DeltaSeconds (`self.SunSpeed`))) false false)
  (`self.UpdateSunDirection`)
  (set `self.IsNight` (`KismetMathLibrary.InRange_FloatFloat` (.pitch (`self.K2_GetActorRotation` _directional_light_actor)) (`self.NightTimeThreshold`) 100.0))
  (if (!= (`self.PreviousNight`) _isnight)
    (set `self.PreviousNight` _isnight)
    (if _isnight
      (`self.Night`)
      (`self.RefreshMaterial`)
      (else
        (`self.Day`)
        (`self.RefreshMaterial`)))))

(event `Night`
  (`LightComponent.SetIntensity` (`Light.LightComponent` (`self.Directional light actor`)) 0.0)
  (set `self.Sun brightness` 0.0)
  (set `self.Stars brightness` 5.0))

(event `Day`
  (`LightComponent.SetIntensity` (`Light.LightComponent` (`self.Directional light actor`)) 3.141593)
  (set `self.Sun brightness` 50.0)
  (set `self.Stars brightness` 1.0))

(fn `UserConstructionScript`
  (`parent.UserConstructionScript`))