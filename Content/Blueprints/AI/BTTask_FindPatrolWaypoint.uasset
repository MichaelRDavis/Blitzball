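; Behavior tree task that picks a random patrol point for a BP_Creature.
; It sets the creature's max speed to patrol speed, then looks for a random reachable point within the patrol radius around the pawn.
; A found point is written to the PatrolLocation blackboard key and the task finishes successfully.
; A failed cast or search never finishes the task, as the current-location fallback is unwired.
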(event `self.ReceiveExecuteAI`
  (params (OwnerController :type "AIController Object Reference") (ControlledPawn :type "Pawn Object Reference"))
  (bind (_randomlocation _returnvalue) (`NavigationSystemV1.K2_GetRandomReachablePointInRadius` (`Actor.K2_GetActorLocation` ControlledPawn) (`self.PatroRadius`) null null))
  (bind _asbp_creature (cast `/Game/Blueprints/AI/BP_Creature` ControlledPawn))
  (`/Game/Blueprints/AI/BP_Creature.SetMaxSpeed` _asbp_creature (`self.PatrolSpeed`))
  (if _returnvalue
    (`BTFunctionLibrary.SetBlackboardValueAsVector` (`self.PatrolLocation`) _randomlocation)
    (`self.FinishExecute` true)))