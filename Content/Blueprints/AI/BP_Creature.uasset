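; BP_Creature is an AI character base with health, a hitscan weapon and death handling.
; Incoming damage lowers Health; at zero it switches the mesh to ragdoll physics, spawns each Shards class at its location and expires after a delay.
; FireWeapon line-traces from the eye viewpoint with debug drawing and damages the hit actor, crediting player controller 0 as instigator.
; SetMaxSpeed exposes walk speed control.
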(event `self.ReceiveAnyDamage`
  (params (Damage :type "Float (single-precision)") (DamageType :type "DamageType Object Reference") (InstigatedBy :type "Controller Object Reference") (DamageCauser :type "Actor Object Reference"))
  (if (and (> Damage 0.0) (not (<= (`self.Health`) 0.0)))
    (set `self.Health` (- (`self.Health`) Damage))
    (if (<= (`self.Health`) 0.0)
      (set `self.IsDead` true)
      (`self.PlayRagdoll`)
      (`self.SpawnShards`)
      (`self.SetLifeSpan` 30.0))))

(event `FireWeapon`
  (bind (_outlocation _outrotation) (`self.GetActorEyesViewPoint`))
  (if (not (`self.IsDead`))
    (bind (_outhit _returnvalue) (`KismetSystemLibrary.LineTraceSingle` _outlocation (+ _outlocation (* (`KismetMathLibrary.GetForwardVector` _outrotation) (`self.WeaponTraceDist`))) "TraceTypeQuery3" true (`|MakeArray` self :!type "Actor Object Reference") "ForDuration"))
    (if _returnvalue
      (`GameplayStatics.ApplyDamage` (`.HitActor` (`GameplayStatics.BreakHitResult` _outhit)) (`self.WeaponDamage`) (`GameplayStatics.GetPlayerController` 0) self))))

(fn `PlayRagdoll`
  (bind _mesh (`self.Mesh`))
  (bind _capsulecomponent (`self.CapsuleComponent`))
  (`PrimitiveComponent.SetAllUseCCD` _mesh true)
  (set `SkinnedMeshComponent.VisibilityBasedAnimTickOption` "AlwaysTickPoseAndRefreshBones" _mesh)
  (`PrimitiveComponent.SetCollisionEnabled` _mesh "QueryAndPhysics")
  (`SkeletalMeshComponent.SetBodyNotifyRigidBodyCollision` _mesh true "None")
  (`PrimitiveComponent.SetSimulatePhysics` _mesh true)
  (`SkeletalMeshComponent.SetAllBodiesPhysicsBlendWeight` _mesh 1.0 false)
  (`PrimitiveComponent.SetCollisionEnabled` _capsulecomponent "NoCollision")
  (`SceneComponent.K2_DetachFromComponent` _capsulecomponent "KeepRelative" "KeepRelative" "KeepRelative" true)
  (`SceneComponent.K2_AttachToComponent` _capsulecomponent (`self.Mesh`) "None" "KeepWorld" "KeepWorld" "KeepWorld" true))

(fn `SetMaxSpeed`
  (params (NewSpeed :type "Float (double-precision)"))
  (set `CharacterMovementComponent.MaxWalkSpeed` NewSpeed (`self.CharacterMovement`)))

(fn `SpawnShards`
  (for _array_element (`self.Shards`)
    (`|SpawnActorFromClass` _array_element (`self.GetTransform`) "AdjustIfPossibleButAlwaysSpawn" "OverrideRootScale" null null)))

(fn `UserConstructionScript`)