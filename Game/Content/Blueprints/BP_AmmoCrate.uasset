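; BP_AmmoCrate is a usable crate that dispenses ammo pickups when the player interacts with it.
; OnUsed spawns every class in the Ammo array at the crate's transform and gives each one's collision component a unit-length impulse in a random direction.
; Focus events toggle custom depth rendering on the crate mesh, typically used for a highlight.
; Nothing here limits reuse or removes the crate afterward.
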(event `self.OnUsed`
  (params (Character :type "FCharacter Object Reference"))
  (for _array_element (`self.Ammo`)
    (bind _returnvalue (`|SpawnActorFromClass` _array_element (`self.GetTransform`) "Undefined" "OverrideRootScale" null null))
    (`PrimitiveComponent.AddImpulseAtLocation` (`FPickup.CollisionComp` _returnvalue) (`KismetMathLibrary.RandomUnitVector`) (0.0 0.0 0.0) "None")))

(event `self.OnBeginFocus`
  (`PrimitiveComponent.SetRenderCustomDepth` (`self.CrateMesh`) true))

(event `self.OnEndFocus`
  (`PrimitiveComponent.SetRenderCustomDepth` (`self.CrateMesh`) false))

(fn `UserConstructionScript`)