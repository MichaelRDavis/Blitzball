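; Projectile actor that deals damage on collision and has a five-second lifespan.
; A sphere collision hit writes the struck actor's name to the visual log, then branches on the sphere's radius.
; A non-positive radius applies point damage; otherwise radial damage spreads from the impact using DamageParams, with Camera as the blocking channel.
; Both paths credit the first player controller as instigator, and the hit does not destroy the projectile.
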(event `self.ReceiveBeginPlay`
  (`self.SetLifeSpan` 5.0))

(event `self.SphereCollisionComp.OnComponentHit`
  (params (HitComponent :type "PrimitiveComponent Object Reference") (OtherActor :type "Actor Object Reference") (OtherComp :type "PrimitiveComponent Object Reference") (NormalImpulse :type "Vector Structure") (Hit :type "HitResult Structure (by ref)"))
  (bind (_bblockinghit _binitialoverlap _time _distance _location _impactpoint _normal _impactnormal _physmat _hitactor) (`GameplayStatics.BreakHitResult` Hit))
  (bind _returnvalue (`GameplayStatics.GetPlayerController` 0))
  (bind (_damageparams_basedamage _damageparams_minimumdamage _damageparams_innerradius _damageparams_outerradius) (break `RadialDamageParams` (`self.DamageParams`)))
  (`VisualLoggerKismetLibrary.LogText` OtherActor (`KismetSystemLibrary.GetDisplayName` OtherActor) "VisLogBP_Projectile" true)
  (if (<= (`SphereComponent.SphereRadius` (`self.SphereCollisionComp`)) 0.0)
    (`GameplayStatics.ApplyPointDamage` _hitactor _damageparams_basedamage _location Hit _returnvalue self)
    (else
      (`GameplayStatics.ApplyRadialDamage` _damageparams_basedamage _location _damageparams_outerradius null (`|MakeArray` self :!type "Actor Object Reference") self _returnvalue false "ECC_Camera"))))

(fn `UserConstructionScript`)