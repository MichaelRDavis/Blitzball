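; BP_Door is a door actor that toggles open and closed when used.
; The OnUsed event flips an IsOpen flag and snaps the DoorMesh relative rotation between closed and a fixed open angle, with no animation.
; BeginPlay and the construction script only call their parent versions.
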(event `self.ReceiveBeginPlay`
  (`parent.ReceiveBeginPlay`))

(event `self.OnUsed`
  (params (Character :type "/Game/Blueprints/Player/BP_Character Object Reference"))
  (if (not (`self.IsOpen`))
    (`SceneComponent.K2_SetRelativeRotation` (`self.DoorMesh`) (struct :`Yaw` -145.0) false false)
    (set `self.IsOpen` true)
    (else
      (`SceneComponent.K2_SetRelativeRotation` :`self` (`self.DoorMesh`))
      (set `self.IsOpen` false))))

(fn `UserConstructionScript`
  (`parent.UserConstructionScript`))