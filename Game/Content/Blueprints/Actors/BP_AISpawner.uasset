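; BP_AISpawner is a placeable actor that spawns AI pawns on a timer, but only at night.
; On BeginPlay it sets a timer, optionally looping, that fires a spawn event.
; The event reads IsNight from the first BP_Sky found in the level and, if true, spawns the configured pawn class with its behavior tree at the spawner's location and rotation.
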(event `self.ReceiveBeginPlay`
  (`KismetSystemLibrary.K2_SetTimerDelegate` (delegate `SpawnAI`) (`self.SpawnTimer`) (`self.Loop`)))

(event `SpawnAI`
  (bind (_returnvalue_location _returnvalue_rotation) (`KismetMathLibrary.BreakTransform` (`self.GetTransform`)))
  (bind _outactors (`GameplayStatics.GetAllActorsOfClass` "/Game/Blueprints/Actors/BP_Sky.BP_Sky_C"))
  (bind _output_get (set `self.CanSpawn` (`/Game/Blueprints/Actors/BP_Sky.IsNight` (`|GetArrayItem` _outactors))))
  (if _output_get
    (`AIBlueprintHelperLibrary.SpawnAIFromClass` (`self.Pawn`) (`self.BehaviorTree`) _returnvalue_location _returnvalue_rotation)))

(fn `UserConstructionScript`)