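; BP_Building is a damageable building actor that destroys itself when its health runs out.
; On BeginPlay it creates and stores a dynamic material instance from the BuildingMesh, which the graph does not use further.
; AnyDamage handles positive damage by setting health to damage minus current health, a reversed subtraction, then destroys the actor at zero or below.
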(event `self.ReceiveBeginPlay`
  (bind _returnvalue (`PrimitiveComponent.CreateDynamicMaterialInstance` (`self.BuildingMesh`) 0 null "None"))
  (set `self.DynamicMaterial` _returnvalue))

(event `self.ReceiveAnyDamage`
  (params (Damage :type "Float (single-precision)") (DamageType :type "DamageType Object Reference") (InstigatedBy :type "Controller Object Reference") (DamageCauser :type "Actor Object Reference"))
  (if (> Damage 0.0)
    (set `self.BuildingHealth` (- Damage (`self.BuildingHealth`)))
    (if (<= (`self.BuildingHealth`) 0.0)
      (`self.K2_DestroyActor`))))

(fn `UserConstructionScript`)