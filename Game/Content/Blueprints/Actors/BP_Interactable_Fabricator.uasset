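; BP_Interactable_Fabricator is an interactable fabricator actor that can spawn items into the world.
; SpawnItem spawns a given class at the SpawnLocation component's world transform, nudging it clear of collisions but always spawning.
; OnUsed is empty; leftover nodes that would add a widget to the viewport, show the cursor and pause the game are disconnected and never run.
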(event `self.OnUsed`
  (params (Character :type "/Game/Blueprints/Player/BP_Character Object Reference")))

(event `SpawnItem`
  (params (Item :type "/Game/Blueprints/Pickups/BP_Pickup Class Reference"))
  (`|SpawnActorFromClass` Item (`SceneComponent.K2_GetComponentToWorld` (`self.SpawnLocation`)) "AdjustIfPossibleButAlwaysSpawn" "OverrideRootScale" null null))

(fn `UserConstructionScript`
  (`parent.UserConstructionScript`))