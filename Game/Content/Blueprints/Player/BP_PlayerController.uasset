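; Player controller that handles the inventory screen, respawning and player leveling.
; The Inventory input opens a new inventory widget, pauses the game and shows the mouse cursor.
; Respawn spawns a new BP_Character at a player start and possesses it.
; LevelUp compares XP to a threshold, then either raises the level, scales the threshold and resets XP, or adds XP to itself.
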(event `InputAction|Inventory`
  (params (Key :type "Key Structure"))
  (:`Pressed`
    (bind _returnvalue (`|CreateWidget` "/Game/UI/Widget_Inventory.Widget_Inventory_C" self))
    (`UserWidget.AddToViewport` _returnvalue 0)
    (`GameplayStatics.SetGamePaused` true)
    (set `self.bShowMouseCursor` true)))

(event `Respawn`
  (bind _returnvalue (`|SpawnActorFromClass` "/Game/Blueprints/Player/BP_Character.BP_Character_C" (`self.GetTransform` (`GameModeBase.K2_FindPlayerStart` (`GameplayStatics.GetGameMode`) self "")) "AdjustIfPossibleButAlwaysSpawn" "OverrideRootScale" null null))
  (`self.Possess` _returnvalue))

(fn `LevelUp`
  (params (XP :type "Float (double-precision)"))
  (if (>= (`self.XP`) (`self.LevelXP`))
    (set `self.PlayerLevel` (+ (`self.PlayerLevel`) 1))
    (set `self.LevelXP` (* (`self.LevelXP`) (`self.LevelXPMultiplier`)))
    (set `self.XP` 0.0)
    (`KismetSystemLibrary.PrintString` "Level Up")
    (else
      (set `self.XP` (+ XP (`self.XP`))))))

(fn `UserConstructionScript`)