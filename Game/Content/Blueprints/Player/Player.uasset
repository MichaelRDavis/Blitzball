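; Player Blueprint that handles weapon selection and helmet light input.
; Number keys 1 to 3 cast the matching Inventory slot to FWeapon and call SwitchWeapon with it and the current Weapon.
; The helmet light starts hidden on BeginPlay, and the F key toggles its visibility through a FlipFlop.
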(event `self.ReceiveBeginPlay`
  (`SceneComponent.SetHiddenInGame` (`self.HelemetLight`) true false))

(event `Key|One`
  (params (Key :type "Key Structure"))
  (:`Pressed`
    (bind _asfweapon (cast `FWeapon` (`|GetArrayItem` (`self.Inventory`))))
    (`self.SwitchWeapon` _asfweapon (`self.Weapon`))))

(event `Key|Two`
  (params (Key :type "Key Structure"))
  (:`Pressed`
    (bind _asfweapon (cast `FWeapon` (`|GetArrayItem` (`self.Inventory`) 1)))
    (`self.SwitchWeapon` _asfweapon (`self.Weapon`))))

(event `Key|Three`
  (params (Key :type "Key Structure"))
  (:`Pressed`
    (bind _asfweapon (cast `FWeapon` (`|GetArrayItem` (`self.Inventory`) 2)))
    (`self.SwitchWeapon` _asfweapon (`self.Weapon`))))

(event `Key|F`
  (params (Key :type "Key Structure"))
  (bind _helemetlight (`self.HelemetLight`))
  (:`Pressed`
    (`/Engine/EditorBlueprintResources/StandardMacros.FlipFlop`
      (:`A`
        (`SceneComponent.SetHiddenInGame` _helemetlight false false))
      (:`B`
        (`SceneComponent.SetHiddenInGame` _helemetlight true false)))))

(fn `UserConstructionScript`)