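; Behavior Tree service that gives the AI a simple sight check against the player character.
; On activation it resets the AI state enum in the blackboard to its default state.
; Each tick it compares the pawn's forward vector with the direction to the player.
; Within a 45-degree half-angle it switches the state and stores the player as enemy, with no distance or line-of-sight test; otherwise it resets the state.
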(event `self.ReceiveActivationAI`
  (params (OwnerController :type "AIController Object Reference") (ControlledPawn :type "Pawn Object Reference"))
  (`BTFunctionLibrary.SetBlackboardValueAsEnum` (`self.AIStateKey`) (enumliteral `/Game/Blueprints/AI/AIState` "NewEnumerator0")))

(event `self.ReceiveTickAI`
  (params (OwnerController :type "AIController Object Reference") (ControlledPawn :type "Pawn Object Reference") (DeltaSeconds :type "Float (single-precision)"))
  (if (< (`KismetMathLibrary.DegAcos` (`KismetMathLibrary.Dot_VectorVector` (`KismetMathLibrary.Normal` (- (`Actor.K2_GetActorLocation` (`GameplayStatics.GetPlayerCharacter` 0)) (`Actor.K2_GetActorLocation` ControlledPawn))) (`Actor.GetActorForwardVector` ControlledPawn))) 45.0)
    (`BTFunctionLibrary.SetBlackboardValueAsEnum` (`self.AIStateKey`) (enumliteral `/Game/Blueprints/AI/AIState` "NewEnumerator1"))
    (`BTFunctionLibrary.SetBlackboardValueAsObject` (`self.EnemyActorKey`) (`GameplayStatics.GetPlayerCharacter` 0))
    (else
      (`BTFunctionLibrary.SetBlackboardValueAsEnum` (`self.AIStateKey`) (enumliteral `/Game/Blueprints/AI/AIState` "NewEnumerator0")))))