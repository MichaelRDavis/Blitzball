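; BP_MonsterAI is the monster's AI controller, running Monster_BehaviorTree and feeding it what AI perception senses about the player.
; Sensing an actor tagged Player cancels the sight timer and sets the line-of-sight and player Blackboard keys.
; Any other perception update, including losing the player or sensing a non-player, starts a timer that clears both keys on expiry, giving the monster a short memory.
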(event `self.ReceiveBeginPlay`
  (`self.RunBehaviorTree` "/Game/Blueprints/AI/Monster_BehaviorTree.Monster_BehaviorTree"))

(event `self.AIPerception.OnTargetPerceptionUpdated`
  (params (Actor :type "Actor Object Reference") (Stimulus :type "AIStimulus Structure"))
  (bind _blackboard (`self.Blackboard`))
  (if (and (`self.ActorHasTag` Actor "Player") (`.bSuccessfullySensed` (break `AIStimulus` Stimulus)))
    (`KismetSystemLibrary.K2_ClearAndInvalidateTimerHandle` (`self.SightTimerHandle`))
    (`BlackboardComponent.SetValueAsBool` _blackboard (`self.HasLineOfSightKey`) true)
    (`BlackboardComponent.SetValueAsObject` _blackboard (`self.PlayerKey`) Actor)
    (else
      (bind _returnvalue (`KismetSystemLibrary.K2_SetTimerDelegate` (delegate `StartSightTimer`) (`self.LineOfSightTimer`)))
      (set `self.SightTimerHandle` _returnvalue))))

(event `StartSightTimer`
  (bind _blackboard (`self.Blackboard`))
  (`BlackboardComponent.SetValueAsBool` _blackboard (`self.HasLineOfSightKey`) false)
  (`BlackboardComponent.SetValueAsObject` _blackboard (`self.PlayerKey`) null))

(fn `UserConstructionScript`)