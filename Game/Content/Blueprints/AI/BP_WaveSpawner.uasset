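; Wave spawner actor that spawns AI Monsters with MonsterBehaviorTree at random navigable points around itself, in waves that grow with the wave count.
; A looping timer spawns one monster at a time until the wave's quota is spent.
; Tick then schedules the next wave after TimeBetweenWaves, unless that timer is already running.
; Its loop over existing monsters' IsDead state does not gate scheduling, so waves can overlap surviving monsters.
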(event `SpawnMonster`
  (bind _returnvalue (`GameplayStatics.GetActorOfClass` "/Script/NavigationSystem.RecastNavMesh"))
  (`AIBlueprintHelperLibrary.SpawnAIFromClass` "/Game/Blueprints/AI/Monster.Monster_C" "/Game/Blueprints/AI/MonsterBehaviorTree.MonsterBehaviorTree" (`NavigationSystemV1.K2_GetRandomLocationInNavigableRadius` (`self.K2_GetActorLocation`) 1000.0 _returnvalue null))
  (bind _result (`/Engine/EditorBlueprintResources/StandardMacros.DecrementFloat` (`self.MonsterCount`))
    (:`  `
      (bind _output_get (set `self.MonsterCount` _result))
      (if (<= _output_get 0.0)
        (`self.EndWave`)))))

(event `StartWave`
  (bind _result (`/Engine/EditorBlueprintResources/StandardMacros.IncrementFloat` (`self.WaveCount`))
    (:`  `
      (bind _output_get (set `self.WaveCount` _result))
      (set `self.MonsterCount` (* _output_get 2.0))
      (bind _returnvalue (`KismetSystemLibrary.K2_SetTimer` null "SpawnMonster" 1.0 true))
      (set `self.SpawnMonsterTimer` _returnvalue))))

(event `EndWave`
  (`KismetSystemLibrary.K2_ClearAndInvalidateTimerHandle` (`self.SpawnMonsterTimer`)))

(event `StartNextWave`
  (bind _returnvalue (`KismetSystemLibrary.K2_SetTimer` null "StartWave" (`self.TimeBetweenWaves`)))
  (set `self.WaveTimer` _returnvalue))

(event `CanSpawnWave`
  (if (`KismetSystemLibrary.K2_IsTimerActiveHandle` (`self.WaveTimer`))
    _
    (elif (<= (`self.MonsterCount`) 0.0)
      (bind _outactors (`GameplayStatics.GetAllActorsOfClass` "/Game/Blueprints/AI/Monster.Monster_C"))
      (for _array_element _outactors
        (if (`FCharacterBase.IsDead` _array_element)
          (break)))
      (`self.StartNextWave`))))

(event `self.ReceiveTick`
  (params (DeltaSeconds :type "Float (single-precision)"))
  (`self.CanSpawnWave`))

(event `self.ReceiveBeginPlay`
  (`self.StartNextWave`))

(fn `UserConstructionScript`)