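; Weapon pickup that gives the using character a weapon spawned from its item class, then destroys itself.
; With more than one inventory item, it drops the current weapon, adds the new one and switches to it.
; Otherwise it only adds the spawned item, with the character set as Instigator.
; Focus events toggle custom depth rendering on the pickup mesh, typically used for highlighting.
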(event `self.OnUsed`
  (params (Character :type "FCharacter Object Reference"))
  (bind _returnvalue (`FCharacter.GetWeapon` Character))
  (if (> (`KismetArrayLibrary.Array_Length` (`FCharacter.Inventory` Character)) 1)
    (`FCharacter.DropItem` Character _returnvalue)
    (bind _returnvalue_2 (`|SpawnActorFromClass` (`self.ItemClass`) (`KismetMathLibrary.MakeTransform` (0.0 0.0 0.0)) "AlwaysSpawn" "OverrideRootScale" null null))
    (`FCharacter.AddItem` Character _returnvalue_2)
    (bind _asfweapon (cast `FWeapon` _returnvalue_2))
    (`FCharacter.SwitchWeapon` Character _asfweapon _returnvalue)
    (`self.K2_DestroyActor`)
    (else
      (bind _returnvalue_3 (`|SpawnActorFromClass` (`self.ItemClass`) (`KismetMathLibrary.MakeTransform` (0.0 0.0 0.0)) "AlwaysSpawn" "OverrideRootScale" null Character))
      (`FCharacter.AddItem` Character _returnvalue_3)
      (`self.K2_DestroyActor`))))

(event `self.OnBeginFocus`
  (`PrimitiveComponent.SetRenderCustomDepth` (`self.PickupMesh`) true))

(event `self.OnEndFocus`
  (`PrimitiveComponent.SetRenderCustomDepth` (`self.PickupMesh`) false))

(fn `UserConstructionScript`)