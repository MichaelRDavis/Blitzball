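; BP_Pickup_Shards is a pickup actor that grants shard currency to the player and expires after a short lifespan.
; When its collision sphere overlaps a BP_Character controlled by a BP_PlayerController, it adds ShardAmount to that controller's Shards and destroys itself.
; The shard total lives on the player controller rather than on the character.
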(event `self.ReceiveBeginPlay`
  (`self.SetLifeSpan` 10.0))

(event `self.SphereCollisionComp.OnComponentBeginOverlap`
  (params (OverlappedComponent :type "PrimitiveComponent Object Reference") (OtherActor :type "Actor Object Reference") (OtherComp :type "PrimitiveComponent Object Reference") (OtherBodyIndex :type Integer) (bFromSweep :type Boolean) (SweepResult :type "HitResult Structure (by ref)"))
  (bind _asbp_character (cast `/Game/Blueprints/Player/BP_Character` OtherActor))
  (bind _asbp_player_controller (cast `/Game/Blueprints/Player/BP_PlayerController` (`Pawn.GetController` _asbp_character)))
  (set `/Game/Blueprints/Player/BP_PlayerController.Shards` (+ (`/Game/Blueprints/Player/BP_PlayerController.Shards` _asbp_player_controller) (`self.ShardAmount`)) _asbp_player_controller)
  (`self.K2_DestroyActor`))

(fn `UserConstructionScript`
  (`parent.UserConstructionScript`))