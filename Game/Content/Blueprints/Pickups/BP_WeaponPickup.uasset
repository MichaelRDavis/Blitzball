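; Weapon pickup that gives the using character a weapon of its item class and then removes itself from the world.
; On use it always adds the item, then checks the character's current weapon to decide whether a swap is needed.
; For a swap it finds the weapon through a world-wide GetActorOfClass lookup, so a failed BP_Weapon cast leaves the pickup in place.
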(event `/Game/Blueprints/Actors/BP_Interactable.OnUsed`
  (params (Character :type "/Game/Blueprints/Player/BP_Character Object Reference"))
  (bind _itemclass (`self.ItemClass`))
  (if (== (`/Game/Blueprints/Player/BP_Character.Weapon` Character) null)
    (`/Game/Blueprints/Player/BP_Character.AddItem` Character _itemclass)
    (`self.K2_DestroyActor`)
    (else
      (`/Game/Blueprints/Player/BP_Character.AddItem` Character _itemclass)
      (bind _returnvalue (`GameplayStatics.GetActorOfClass` _itemclass))
      (bind _asbp_weapon (cast `/Game/Blueprints/Weapons/BP_Weapon` _returnvalue))
      (`/Game/Blueprints/Player/BP_Character.SwapWeapon` Character _asbp_weapon)
      (`self.K2_DestroyActor`))))

(fn `UserConstructionScript`
  (`parent.UserConstructionScript`))