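; Monster Blueprint for an armed enemy that awards kill XP to the player when destroyed.
; On BeginPlay it spawns its weapon, takes ownership and attaches the weapon mesh to its own mesh at the weapon-defined hands socket.
; FireWeapon spawns the weapon's projectile class at the Muzzle socket.
; Destroyed passes KillXP to player 0's FPlayerState LevelUp, then destroys the weapon, both only if the player casts succeed.
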(event `self.ReceiveBeginPlay`
  (`self.AddWeapon`))

(event `AddWeapon`
  (bind _returnvalue (`|SpawnActorFromClass` (`self.Weapon`) (`KismetMathLibrary.MakeTransform` (0.0 0.0 0.0)) "AlwaysSpawn" "OverrideRootScale" null self))
  (bind _output_get (set `self.Weap` _returnvalue))
  (`self.SetOwner` _returnvalue self)
  (`self.SetOwner` _output_get self)
  (`SceneComponent.K2_AttachToComponent` (`FWeapon.Mesh` _returnvalue) (`self.Mesh`) (`FWeapon.HandsAttachSocket` _returnvalue) "SnapToTarget" "SnapToTarget" "SnapToTarget" true))

(event `FireWeapon`
  (`|SpawnActorFromClass` (`FWeapon.ProjectileClass` (`self.Weap`)) (`SceneComponent.GetSocketTransform` (`FWeapon.Mesh` (`self.Weap`)) "Muzzle" "RTS_World") "AdjustIfPossibleButAlwaysSpawn" "OverrideRootScale" null self))

(event `self.ReceiveDestroyed`
  (bind _asfplayer_controller (cast `FPlayerController` (`GameplayStatics.GetPlayerController` 0)))
  (bind _asfplayer_state (cast `FPlayerState` (`Controller.PlayerState` _asfplayer_controller)))
  (`FPlayerState.LevelUp` _asfplayer_state (`self.KillXP`))
  (`self.K2_DestroyActor` (`self.Weap`)))

(fn `UserConstructionScript`)