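; Weapon pickup actor that, when used, spawns its item class, adds it to the using character and destroys itself.
; If the character's weapon check passes, it sets the character as instigator and equips the spawned item as a weapon.
; In that branch, a failed weapon cast leaves the pickup in the world.
; Focus events toggle custom depth rendering on the pickup mesh.
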(event `self.OnUsed`
  (params (Character :type "FCharacter Object Reference"))
  (if (== (`FCharacter.Weapon` Character) null)
    (bind _returnvalue (`|SpawnActorFromClass` (`self.ItemClass`) (`KismetMathLibrary.MakeTransform` (0.0 0.0 0.0)) "AlwaysSpawn" "OverrideRootScale" null Character))
    (`FCharacter.AddItem` Character _returnvalue)
    (bind _asfweapon (cast `FWeapon` _returnvalue)) ; Equip item if it is a weapon
    (`FCharacter.EquipWeapon` Character _asfweapon)
    (`self.K2_DestroyActor`)
    (else
      (bind _returnvalue_2 (`|SpawnActorFromClass` (`self.ItemClass`) (`KismetMathLibrary.MakeTransform` (0.0 0.0 0.0)) "AlwaysSpawn" "OverrideRootScale" null null))
      (`FCharacter.AddItem` Character _returnvalue_2)
      (`self.K2_DestroyActor`))))

(event `self.OnBeginFocus`
  (`PrimitiveComponent.SetRenderCustomDepth` (`self.PickupMesh`) true))

(event `self.OnEndFocus`
  (`PrimitiveComponent.SetRenderCustomDepth` (`self.PickupMesh`) false))

(fn `UserConstructionScript`)