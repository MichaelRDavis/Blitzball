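; Fabricator is an interactable actor that opens the Fabricator UI widget when used.
; OnUsed creates the widget for player 0, adds it to the viewport, shows the mouse cursor and switches input to UI only with the widget focused.
; Focus events toggle custom depth rendering on the mesh to mark it while the actor is focused.
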(event `self.OnUsed`
  (params (Character :type "FCharacter Object Reference"))
  (bind _returnvalue (`GameplayStatics.GetPlayerController` 0))
  (bind _returnvalue_2 (`|CreateWidget` "/Game/UI/Fabricator.Fabricator_C" _returnvalue))
  (`UserWidget.AddToViewport` _returnvalue_2 0)
  (set `PlayerController.bShowMouseCursor` true _returnvalue)
  (`WidgetBlueprintLibrary.SetInputMode_UIOnlyEx` _returnvalue _returnvalue_2))

(event `self.OnBeginFocus`
  (`PrimitiveComponent.SetRenderCustomDepth` (`self.FabricatorMesh`) true))

(event `self.OnEndFocus`
  (`PrimitiveComponent.SetRenderCustomDepth` (`self.FabricatorMesh`) false))

(fn `UserConstructionScript`)