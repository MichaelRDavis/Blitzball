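; A usable loot crate that drops a single pickup of its DropType class the first time a character uses it.
; OnUsed calls Spawn, which creates the drop at the Scene component's transform and tosses its PickupMesh with a randomized velocity-change impulse.
; A HasBeenOpened flag limits it to one drop, with later uses printing an empty message.
; Focus events toggle custom depth rendering on the crate mesh.
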(event `self.OnUsed`
  (params (Character :type "FCharacter Object Reference"))
  (`self.Spawn` Character))

(event `Spawn`
  (params (Character :type "FCharacter Object Reference"))
  (if (not (`self.HasBeenOpened`))
    (bind _returnvalue (`|SpawnActorFromClass` (`self.DropType`) (`SceneComponent.K2_GetComponentToWorld` (`self.Scene`)) "AdjustIfPossibleButAlwaysSpawn" "OverrideRootScale" null null))
    (set `self.HasBeenOpened` true)
    (`PrimitiveComponent.AddImpulse` (`FPickup.PickupMesh` _returnvalue) (`KismetMathLibrary.MakeVector` (`KismetMathLibrary.RandomFloatInRange` -50.0 100.0) (`KismetMathLibrary.RandomFloatInRange` -50.0 100.0) (`KismetMathLibrary.RandomFloatInRange` -250.0 500.0)) "None" true)
    (else
      (`KismetSystemLibrary.PrintString` "Crate empty"))))

(event `self.OnBeginFocus`
  (`PrimitiveComponent.SetRenderCustomDepth` (`self.CrateMesh`) true))

(event `self.OnEndFocus`
  (`PrimitiveComponent.SetRenderCustomDepth` (`self.CrateMesh`) false))

(fn `UserConstructionScript`)