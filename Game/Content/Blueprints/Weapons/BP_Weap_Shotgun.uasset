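; BP_Weap_Shotgun is a shotgun weapon Blueprint that fires multiple instant-hit shots each time it fires.
; Its Fire event runs the parent logic, then loops over a range set by AmmoCost, calling FireInstantHit on each pass, so the shot count follows the ammo cost.
; BeginPlay, StartFire, StopFire and the construction script only pass through to the parent class.
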(event `self.ReceiveBeginPlay`
  (`parent.ReceiveBeginPlay`))

(event `self.Fire`
  (`parent.Fire`)
  (for _ (range (+ (`self.AmmoCost`) 1))
    (`self.FireInstantHit`)))

(event `self.StartFire`
  (`parent.StartFire`))

(event `self.StopFire`
  (`parent.StopFire`))

(fn `UserConstructionScript`
  (`parent.UserConstructionScript`))