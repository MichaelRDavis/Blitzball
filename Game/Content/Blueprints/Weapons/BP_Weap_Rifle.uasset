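; BP_Weap_Rifle is an automatic rifle weapon that fires instant-hit shots while firing is active.
; StartFire changes the weapon state and starts a looping timer that calls Fire every FireRate seconds, so the first shot lands one interval later.
; Each Fire runs the parent's logic, then FireInstantHit.
; StopFire switches the weapon state and clears the stored timer handle.
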(event `self.ReceiveBeginPlay`
  (`parent.ReceiveBeginPlay`))

(event `self.Fire`
  (`parent.Fire`)
  (`self.FireInstantHit`))

(event `self.StartFire`
  (`self.SetWeaponState` "NewEnumerator1")
  (bind _returnvalue (`KismetSystemLibrary.K2_SetTimer` null "Fire" (`self.FireRate`) true))
  (set `self.FiringHandle` _returnvalue))

(event `self.StopFire`
  (`self.SetWeaponState` "NewEnumerator0")
  (`KismetSystemLibrary.K2_ClearAndInvalidateTimerHandle` (`self.FiringHandle`)))

(fn `UserConstructionScript`
  (`parent.UserConstructionScript`))