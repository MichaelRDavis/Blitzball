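; BP_ForceGun is a weapon Blueprint meant to push characters it is fired at.
; Firing runs a visibility line trace, with debug drawing, from the owner's eye viewpoint along the view direction out to ForceRange.
; A blocking hit on a character adds an impulse to its first found primitive component at the impact point and bone.
; The impulse is currently a zero vector, so it applies no push.
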(event `self.K2_Fire`
  (`self.ApplyForce`))

(event `ApplyForce`
  (bind (_outlocation _outrotation) (`self.GetActorEyesViewPoint` (`self.FOwner`)))
  (bind _outhit (`KismetSystemLibrary.LineTraceSingle` :`Start` _outlocation :`End` (+ _outlocation (* (`KismetMathLibrary.GetForwardVector` _outrotation) (`self.ForceRange`))) :`TraceChannel` "TraceTypeQuery1" :`DrawDebugType` "ForDuration"))
  (bind (_bblockinghit _binitialoverlap _time _distance _location _impactpoint _normal _impactnormal _physmat _hitactor _hitcomponent _hitbonename) (`GameplayStatics.BreakHitResult` _outhit))
  (if _bblockinghit
    (bind _asfcharacter (cast `FCharacter` _hitactor))
    (`/Engine/EditorBlueprintResources/StandardMacros.IsValid` _asfcharacter
      (:`Is Valid`
        (`PrimitiveComponent.AddImpulseAtLocation` (`self.GetComponentByClass` _asfcharacter "/Script/Engine.PrimitiveComponent") (0.0 0.0 0.0) _impactpoint _hitbonename)))))

(fn `UserConstructionScript`)