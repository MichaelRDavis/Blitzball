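; Base first-person weapon actor that handles ammo, firing state, attachment to the owner's hands and fire montage and sound.
; Fire only plays effects and spends ammo; separate hitscan and projectile functions are provided but not called here.
; Hitscan traces from the camera within a targeting-dependent spread cone, applies recoil, head-bone bonus damage and impulse.
; Reload adjusts magazine ammo immediately before its delay, and CanReload always returns false.
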(event `self.ReceiveBeginPlay`
  (`self.SetWeaponState` "NewEnumerator0")
  (if (> (`self.Mags`) 0)
    (set `self.MagAmmo` (`self.MaxMagAmmo`))
    (set `self.Ammo` (* (`self.MagAmmo`) (`self.Mags`)))))

(event `Fire`
  (if (> (`self.MagAmmo`) 0)
    (`self.SimulateWeaponFire`)
    (`self.UseAmmo`)))

(event `StartFire`
  (`self.Fire`)
  (`self.SetWeaponState` "NewEnumerator1"))

(event `StopFire`
  (`self.SetWeaponState` "NewEnumerator0"))

(event `ReloadWeapon`
  (set `self.IsReloading` false)
  (`self.Reload`)
  (`KismetSystemLibrary.Delay` (`self.ReloadTIme`))
  (set `self.IsReloading` false))

(fn `AddAmmo`
  (params (AmmoAmount :type Integer))
  (returns (Ammo :type Integer))
  (locals (AmmoDelta :type Integer))
  (bind _output_get (set `local.AmmoDelta` (`KismetMathLibrary.Max` (- (`self.MaxAmmo`) (`self.Ammo`)))))
  (set `self.Ammo` (+ (`KismetMathLibrary.Min` _output_get AmmoAmount) 1))
  (return (`KismetMathLibrary.Max` 0 (- AmmoAmount (`local.AmmoDelta`)))))

(fn `ApplyRecoil`
  (bind _pawnowner (`self.PawnOwner`))
  (if (== (`self.WeaponState`) (enumliteral `/Game/Blueprints/Weapons/EWeaponState` "NewEnumerator1"))
    (set `self.VerticalRecoil` (`KismetMathLibrary.RandomFloatInRange` 0.0 -0.5))
    (set `self.HorizontalRecoil` (`KismetMathLibrary.RandomFloatInRange` -0.5 0.5))
    (`Pawn.AddControllerPitchInput` _pawnowner (`self.VerticalRecoil`))
    (`Pawn.AddControllerYawInput` _pawnowner (`self.HorizontalRecoil`))))

(fn `AttachToOwner`
  (`SceneComponent.K2_AttachToComponent` (`self.WeaponMesh`) (`/Game/Blueprints/Player/BP_Character.FirstPersonMesh` (`self.PawnOwner`)) (`self.HandsAttachSocket`) "SnapToTarget" "SnapToTarget" "SnapToTarget" true))

(fn `CanFire`
  (returns (CanFire :type Boolean))
  (return (or (== (`self.WeaponState`) (enumliteral `/Game/Blueprints/Weapons/EWeaponState` "NewEnumerator0")) (== (`self.WeaponState`) (enumliteral `/Game/Blueprints/Weapons/EWeaponState` "NewEnumerator1")))))

(fn `CanReload`
  (returns (GotAmmo :type Boolean))
  (return false))

(fn `DetachFromOwner`
  (`SceneComponent.K2_DetachFromComponent` (`self.WeaponMesh`) "KeepRelative" "KeepRelative" "KeepRelative" true))

(fn `FireInstantHit`
  (locals (CurrentSpread :type "Float (double-precision)"))
  (bind _pawnowner (`self.PawnOwner`))
  (bind _charactercameracomponent (`/Game/Blueprints/Player/BP_Character.CharacterCameraComponent` _pawnowner))
  (bind _returnvalue (`SceneComponent.K2_GetComponentLocation` _charactercameracomponent))
  (if (`/Game/Blueprints/Player/BP_Character.GetIsTargeting` _pawnowner)
    (set `local.CurrentSpread` (`self.TargetingSpread`))
    (else
      (set `local.CurrentSpread` (`self.Spread`))))
  (`self.ApplyRecoil`)
  (bind (_outhit _returnvalue_2) (`KismetSystemLibrary.LineTraceSingle` _returnvalue (+ _returnvalue (* (`KismetMathLibrary.RandomUnitVectorInConeInDegrees` (`KismetMathLibrary.GetForwardVector` (`SceneComponent.K2_GetComponentRotation` _charactercameracomponent)) (`local.CurrentSpread`)) (`self.MaxTraceDist`))) "TraceTypeQuery3" true (`|MakeArray` self (`self.PawnOwner`) :!type "Actor Object Reference")))
  (if _returnvalue_2
    (bind (_bblockinghit _binitialoverlap _time _distance _location _impactpoint _normal _impactnormal _physmat _hitactor _hitcomponent _hitbonename) (`GameplayStatics.BreakHitResult` _outhit))
    (if (== _hitbonename "head")
      ;[0 0 0] Replace with physical material headshot damage
      (`GameplayStatics.ApplyDamage` _hitactor (* (`self.HeadshotMultiplier`) (`self.Damage`)) (`GameplayStatics.GetPlayerController` 0) self)
      (`/Engine/EditorBlueprintResources/StandardMacros.IsValid` _hitcomponent
        (:`Is Valid`
          (`PrimitiveComponent.AddImpulseAtLocation` _hitcomponent (* _location (`self.ImpulseVelcoity`)) _location _hitbonename)))
      (else
        (`GameplayStatics.ApplyDamage` _hitactor (`self.Damage`) (`GameplayStatics.GetPlayerController` 0) self)
        (`/Engine/EditorBlueprintResources/StandardMacros.IsValid` _hitcomponent
          (:`Is Valid`
            (`PrimitiveComponent.AddImpulseAtLocation` _hitcomponent (* _location (`self.ImpulseVelcoity`)) _location _hitbonename)))))))

(fn `FireProjectile`
  (bind _weaponmesh (`self.WeaponMesh`))
  (`|SpawnActorFromClass` (`self.ProjectileClass`) (`SceneComponent.GetSocketTransform` _weaponmesh (`SkinnedMeshComponent.GetSocketBoneName` _weaponmesh (`self.MuzzeLocation`)) "RTS_World") "AlwaysSpawn" "OverrideRootScale" self (`self.PawnOwner`)))

(fn `Reload`
  (locals (MagDelta :type Integer))
  (bind _output_get (set `local.MagDelta` (`KismetMathLibrary.Min` (- (`self.MaxMagAmmo`) (`self.MagAmmo`)) (- (`self.Ammo`) (`self.MagAmmo`)))))
  (if (> _output_get 0)
    (set `self.MagAmmo` (+ (`local.MagDelta`) 1))))

(fn `SetWeaponOwner`
  (params (NewOwner :type "/Game/Blueprints/Player/BP_Character Object Reference"))
  (`/Engine/EditorBlueprintResources/StandardMacros.IsValid` NewOwner
    (:`Is Valid`
      (`self.SetOwner` NewOwner NewOwner)
      (set `self.Instigator` NewOwner)
      (set `self.PawnOwner` NewOwner))))

(fn `SetWeaponState`
  (params (NewState :type "/Game/Blueprints/Weapons/EWeaponState Enum" :default "NewEnumerator0"))
  (set `self.WeaponState` NewState))

(fn `SimulateWeaponFire`
  (`AnimInstance.Montage_Play` (`SkeletalMeshComponent.GetAnimInstance` (`/Game/Blueprints/Player/BP_Character.FirstPersonMesh` (`self.PawnOwner`))) "/Game/FirstPerson/Animations/FirstPersonFire_Montage.FirstPersonFire_Montage" 1.0 "MontageLength" 0.0 true)
  (`GameplayStatics.SpawnSoundAttached` (`self.FireSound`) (`self.WeaponMesh`) "None" (0.0 0.0 0.0) (struct) "KeepRelativeOffset" false 1.0 1.0 0.0 null null))

(fn `UseAmmo`
  (bind _result (`/Engine/EditorBlueprintResources/StandardMacros.DecrementInt` (`self.MagAmmo`))
    (:`  `
      (set `self.MagAmmo` _result)
      (bind _result_2 (`/Engine/EditorBlueprintResources/StandardMacros.DecrementInt` (`self.Ammo`))
        (:`  `
          (set `self.Ammo` _result_2))))))

(fn `UserConstructionScript`
  (`parent.UserConstructionScript`))