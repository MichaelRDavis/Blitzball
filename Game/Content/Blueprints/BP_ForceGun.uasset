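; BP_ForceGun is a gun Blueprint that pushes physics objects with a radial impulse when fired.
; Fire calls ApplyForce, which line traces on the Camera channel from the player's eye view point along the view direction, with timed debug drawing.
; On a hit, it adds a constant-falloff, velocity-change radial impulse to the hit component at the impact point.
; AttachToOwner and DetachFromOwner are empty.
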(event `Fire`
  (`self.ApplyForce`))

(fn `ApplyForce`
  (bind (_outlocation _outrotation) (`self.GetActorEyesViewPoint` (`self.Player`)))
  (bind (_outhit _returnvalue) (`KismetSystemLibrary.LineTraceSingle` :`Start` _outlocation :`End` (+ _outlocation (* (`KismetMathLibrary.GetForwardVector` _outrotation) (`self.TraceDist`))) :`TraceChannel` "TraceTypeQuery2" :`DrawDebugType` "ForDuration"))
  (if _returnvalue
    (bind (_bblockinghit _binitialoverlap _time _distance _location _impactpoint _normal _impactnormal _physmat _hitactor _hitcomponent) (`GameplayStatics.BreakHitResult` _outhit))
    (`PrimitiveComponent.AddRadialImpulse` _hitcomponent _impactpoint (`self.ForceRadius`) (`self.ForceImpulse`) "RIF_Constant" true)))

(fn `AttachToOwner`)

(fn `DetachFromOwner`)

(fn `UserConstructionScript`)