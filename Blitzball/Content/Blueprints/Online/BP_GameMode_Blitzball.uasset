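; Game mode for Blitzball that puts joining players on teams and picks their spawn points.
; On PostLogin, ChooseTeam scans the other players' teams, aiming at the least populated with a random tie-break, and the result is set on the BP_PlayerState.
; Its random pick converts an index into the candidate list directly to a team value, not the stored element.
; FindPlayerStart returns the first BP_PlayerStart whose team matches the player's.
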(event `self.K2_PostLogin`
  (params (NewPlayer :type "PlayerController Object Reference"))
  (bind _asbp_player_state (cast `/Game/Blueprints/Online/BP_PlayerState` (`Controller.PlayerState` NewPlayer)))
  (bind _team (`self.ChooseTeam` _asbp_player_state))
  (`/Game/Blueprints/Online/BP_PlayerState.SetTeam` _asbp_player_state _team))

(fn `ChooseTeam`
  (params (PlayerState :type "/Game/Blueprints/Online/BP_PlayerState Object Reference"))
  (returns (Team :type "/Game/Blueprints/Player/ETeam Enum"))
  (locals (Teams :type "Array of Byte") (BestTeamCount :type Integer :default 0) (BestTeam :type "Array of Byte") (BestRandTeam :type Byte))
  (for _array_element (`GameStateBase.PlayerArray` (`GameplayStatics.GetGameState`))
    (bind _asbp_player_state (cast `/Game/Blueprints/Online/BP_PlayerState` _array_element))
    (if (and (!= _asbp_player_state PlayerState) (`KismetArrayLibrary.Array_IsValidIndex` (`local.Teams`) (`KismetMathLibrary.Conv_ByteToInt` (`/Game/Blueprints/Online/BP_PlayerState.Team` _asbp_player_state))))
      (bind _returnvalue (`KismetArrayLibrary.Array_Add` (`local.Teams`) (`/Game/Blueprints/Online/BP_PlayerState.Team` _asbp_player_state)))
      (bind _output_get (set `local.BestTeamCount` _returnvalue))
      (for (_ _array_index) (`local.Teams`)
        (if (> _output_get _array_index)
          (set `local.BestTeamCount` _array_index)
          (for (_array_element_2 _array_index_2) (`local.Teams`)
            (if (== _array_index_2 (`local.BestTeamCount`))
              (`KismetArrayLibrary.Array_Add` (`local.BestTeam`) _array_element_2)
              (bind _output_get_2 (set `local.BestRandTeam` (`KismetMathLibrary.Conv_IntToByte` (`KismetMathLibrary.RandomInteger` (`KismetArrayLibrary.Array_Length` (`local.BestTeam`))))))
              (return (cast `/Game/Blueprints/Player/ETeam` _output_get_2)))))))))

(fn `FindPlayerStart`
  (params (Player :type "Controller Object Reference") (IncomingName :type String))
  (returns (ReturnValue :type "Actor Object Reference"))
  (bind _asbp_player_state (cast `/Game/Blueprints/Online/BP_PlayerState` (`Controller.PlayerState` Player)))
  (bind _outactors (`GameplayStatics.GetAllActorsOfClass` "/Game/Blueprints/Player/BP_PlayerStart.BP_PlayerStart_C"))
  (for _array_element _outactors
    (if (`|EnumEquality` (`/Game/Blueprints/Player/BP_PlayerStart.Team` _array_element) (`/Game/Blueprints/Online/BP_PlayerState.Team` _asbp_player_state))
      (return _array_element))))

(fn `UserConstructionScript`
  (`parent.UserConstructionScript`))