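; Player Blueprint that hooks up its widget and toggles a scoreboard while Tab is held.
; On BeginPlay it casts the user widget object of its Widget component to Widget_Player and hands it a reference to itself.
; Each Tab press creates a new Widget_Scoreboard for player controller 0 and adds it to the viewport, and release removes it from its parent.
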(event `self.ReceiveBeginPlay`
  (bind _aswidget_player (cast `/Game/UI/HUD/Widget_Player` (`WidgetComponent.GetUserWidgetObject` (`self.Widget`))))
  (set `/Game/UI/HUD/Widget_Player.Player` self _aswidget_player))

(event `Key|Tab`
  (params (Key :type "Key Structure"))
  (:`Pressed`
    (bind _returnvalue (`|CreateWidget` "/Game/UI/HUD/Widget_Scoreboard.Widget_Scoreboard_C" (`GameplayStatics.GetPlayerController` 0)))
    (bind _output_get (set `self.ScoreboardWidget` _returnvalue))
    (`UserWidget.AddToViewport` _output_get 0))
  (:`Released`
    (`Widget.RemoveFromParent` (`self.ScoreboardWidget`))))

(fn `UserConstructionScript`)