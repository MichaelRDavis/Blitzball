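; Player blueprint that shoots the ball it currently possesses.
; On begin play it casts its widget component's user widget to Widget_Player and hands it a reference to itself.
; Right mouse or the Shoot event applies a strong forward and upward impulse to the possessed ball's collision component, if valid, and plays a shoot sound at the player's location.
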(event `self.ReceiveBeginPlay`
  (bind _aswidget_player (cast `/Game/UI/HUD/Widget_Player` (`WidgetComponent.GetUserWidgetObject` (`self.Widget`))))
  (set `/Game/UI/HUD/Widget_Player.Player` self _aswidget_player))

(event `Shoot`
  (bind _returnvalue (`self.GetPossesedBall`))
  (`/Engine/EditorBlueprintResources/StandardMacros.IsValid` _returnvalue
    (:`Is Valid`
      (`PrimitiveComponent.AddImpulse` (`BBlitzball.CollisionComp` _returnvalue) (* (+ (`self.GetActorForwardVector`) (`KismetMathLibrary.MakeVector` 0.0 0.0 0.5)) 500000.0) "None" false)
      (`GameplayStatics.PlaySoundAtLocation` "/Game/Sounds/SoundCue_BallShoot.SoundCue_BallShoot" (`self.K2_GetActorLocation`) (struct) 1.0 1.0 0.0 null null null))))

(event `Key|RightMouseButton`
  (params (Key :type "Key Structure"))
  (:`Pressed`
    (`self.Shoot`)))

(fn `UserConstructionScript`)