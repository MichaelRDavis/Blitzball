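; Game mode Blueprint for Blitzball, with an apparently unfinished start on assigning players to teams.
; PostLogin only casts the new player's state to BP_PlayerState and does nothing further.
; FindTeam appends a zero to Teams, then scans PlayerArray and sets the first player whose team is a valid Teams index to the team in the first entry.
; Nothing in this Blueprint calls FindTeam.
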(event `self.K2_PostLogin`
  (params (NewPlayer :type "PlayerController Object Reference"))
  (cast `/Game/Blueprints/Online/BP_PlayerState` (`Controller.PlayerState` NewPlayer)))

(fn `FindTeam`
  (returns (TeamNumber :type Integer))
  (locals (Teams :type "Array of Integer") (Player :type "/Game/Blueprints/Online/BP_PlayerState Object Reference"))
  (`KismetArrayLibrary.Array_Add` (`local.Teams`))
  (for (_ _array_index) (`GameStateBase.PlayerArray` (`GameplayStatics.GetGameState`))
    (bind _asbp_player_state (cast `/Game/Blueprints/Online/BP_PlayerState` (`|GetArrayItem` (`GameStateBase.PlayerArray` (`GameplayStatics.GetGameState`)) _array_index)))
    (bind _output_get (set `local.Player` _asbp_player_state))
    (if (`KismetArrayLibrary.Array_IsValidIndex` (`local.Teams`) (`KismetMathLibrary.Conv_ByteToInt` (`KismetSystemLibrary.MakeLiteralByte` (`/Game/Blueprints/Online/BP_PlayerState.Team` (`local.Player`)))))
      (`/Game/Blueprints/Online/BP_PlayerState.SetTeam` _output_get (cast `/Game/Blueprints/Player/ETeam` (`KismetMathLibrary.Conv_IntToByte` (`|GetArrayItem` (`local.Teams`)))))
      (return 0))))

(fn `UserConstructionScript`
  (`parent.UserConstructionScript`))