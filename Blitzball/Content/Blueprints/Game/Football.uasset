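; Football actor that plays bounce sounds and lets airborne players head the ball.
; On hit, PlayHitSound plays a bounce for non-player contacts when velocity differs enough from the last stored value, which updates only then.
; ServerHeaderBall calls HeaderBall, which checks for a head-bone contact through the player's physics asset.
; A header applies an impulse along control rotation, using the contact normal as its location, and plays a sound.
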(event `self.ReceiveHit`
  (params (MyComp :type "PrimitiveComponent Object Reference") (Other :type "Actor Object Reference") (OtherComp :type "PrimitiveComponent Object Reference") (bSelfMoved :type Boolean) (HitLocation :type "Vector Structure") (HitNormal :type "Vector Structure") (NormalImpulse :type "Vector Structure") (Hit :type "HitResult Structure (by ref)"))
  (`self.PlayHitSound` MyComp Other)
  (`self.ServerHeaderBall` Other HitLocation))

(event `ServerHeaderBall`
  (params (Actor :type "Actor Object Reference") (Location :type "Vector Structure"))
  (`self.HeaderBall` Actor Location))

(fn `HeaderBall`
  (params (Actor :type "Actor Object Reference") (Location :type "Vector Structure"))
  (bind _asplayer (cast `/Game/Blueprints/Player/Player` Actor))
  (bind (_closestworldposition _normal _bonename) (`SkeletalMeshComponent.K2_GetClosestPointOnPhysicsAsset` (`Character.Mesh` _asplayer) Location))
  (if (and (not (`NavMovementComponent.IsMovingOnGround` (`Character.CharacterMovement` _asplayer))) (== _bonename "head"))
    (`PrimitiveComponent.AddImpulseAtLocation` (`self.CollisionComp`) (* (`KismetMathLibrary.GetForwardVector` (`Pawn.GetControlRotation` _asplayer)) 20000.0) _normal "None")
    (`GameplayStatics.PlaySoundAtLocation` "/Game/Sounds/SoundCue_HeaderSound.SoundCue_HeaderSound" (`self.K2_GetActorLocation`) (struct) 1.0 1.0 0.0 null null null)))

(fn `PlayHitSound`
  (params (OtherComp :type "PrimitiveComponent Object Reference") (OtherActor :type "Actor Object Reference"))
  (locals (LastVelocity :type "Vector Structure"))
  (if (not (`self.ActorHasTag` OtherActor "Player"))
    (bind _returnvalue (`PrimitiveComponent.GetPhysicsLinearVelocity` OtherComp "None"))
    (if (> (`KismetMathLibrary.VSize` (- _returnvalue (`local.LastVelocity`))) 500.0)
      (set `local.LastVelocity` _returnvalue)
      (`GameplayStatics.PlaySoundAtLocation` "/Game/Sounds/SoundCue_BallBounce.SoundCue_BallBounce" (`self.K2_GetActorLocation`) (struct) 1.0 1.0 0.0 null null null))))

(fn `UserConstructionScript`)