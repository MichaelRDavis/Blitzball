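; Goal Blueprint for a Blitzball game that awards save points through its SaveBox overlap volume.
; On overlap it casts the same overlapping actor to both BCharacter and BBlitzball, so both casts must succeed to continue.
; If the character's player state matches the goal's team number and the ball is flagged as hit, that player state scores a save.
; The goal effects event is an empty stub.
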(event `self.SaveBox.OnComponentBeginOverlap`
  (params (OverlappedComponent :type "PrimitiveComponent Object Reference") (OtherActor :type "Actor Object Reference") (OtherComp :type "PrimitiveComponent Object Reference") (OtherBodyIndex :type Integer) (bFromSweep :type Boolean) (SweepResult :type "HitResult Structure (by ref)"))
  (bind _asbcharacter (cast `BCharacter` OtherActor))
  (bind _asbblitzball (cast `BBlitzball` OtherActor))
  (`/Engine/EditorBlueprintResources/StandardMacros.IsValid` _asbblitzball
    (:`Is Valid`
      (bind _asbplayer_state (cast `BPlayerState` (`Pawn.PlayerState` _asbcharacter)))
      (if (and (== (`BPlayerState.GetTeamNumber` _asbplayer_state) (`self.TeamNumber`)) (`BBlitzball.bIsHit` _asbblitzball))
        (`BPlayerState.ScoreSave` _asbplayer_state _asbplayer_state 50)))))

(event `self.OnPlayGoalEffects`)

(fn `UserConstructionScript`)