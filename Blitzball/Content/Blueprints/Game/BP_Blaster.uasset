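; BP_Blaster is a first-person weapon that pushes physics objects with a radial impulse at the point it hits.
; GiveTo and Remove set or clear owner and instigator, while EquipWeapon snaps the mesh to the owner's first-person hands socket.
; Fire runs a debug-drawn complex line trace from the owner's eyes, applying the velocity-change impulse to the hit component.
; AltFire is empty, and DetachFromOwner detaches the owner's Mesh, not the blaster's.
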(event `Fire`
  (`self.FireBlast`))

(event `AltFire`)

(fn `AttachToOwner`
  (`SceneComponent.K2_AttachToComponent` (`self.Mesh`) (`/Game/Blueprints/Player/BP_Player.FirstPersonMesh` (`self.PlayerOwner`)) (`self.HandsAttachSocket`) "SnapToTarget" "SnapToTarget" "SnapToTarget" true))

(fn `DetachFromOwner`
  (`SceneComponent.K2_DetachFromComponent` (`Character.Mesh` (`self.PlayerOwner`)) "KeepRelative" "KeepRelative" "KeepRelative" true))

(fn `EquipWeapon`
  (`self.AttachToOwner`))

(fn `FireBlast`
  (bind (_outlocation _outrotation) (`self.GetActorEyesViewPoint` (`self.PlayerOwner`)))
  (bind (_outhit _returnvalue) (`KismetSystemLibrary.LineTraceSingle` _outlocation (+ _outlocation (* (`KismetMathLibrary.GetForwardVector` _outrotation) (`self.TraceDistance`))) "TraceTypeQuery3" true (`|MakeArray` (`self.PlayerOwner`) :!type "Actor Object Reference") "ForDuration"))
  (if _returnvalue
    (bind (_bblockinghit _binitialoverlap _time _distance _location _impactpoint _normal _impactnormal _physmat _hitactor _hitcomponent) (`GameplayStatics.BreakHitResult` _outhit))
    (`PrimitiveComponent.AddRadialImpulse` _hitcomponent _location 500.0 (`self.BlasterImpulse`) "RIF_Linear" true)))

(fn `GiveTo`
  (params (`New Owner` :type "/Game/Blueprints/Player/BP_Player Object Reference"))
  (bind _output_get (set `self.PlayerOwner` `New Owner`))
  (bind _output_get_2 (set `self.Instigator` _output_get))
  (`self.SetOwner` _output_get_2))

(fn `Remove`
  (set `self.PlayerOwner` null)
  (set `self.Instigator` null)
  (`self.SetOwner` null))

(fn `UserConstructionScript`)