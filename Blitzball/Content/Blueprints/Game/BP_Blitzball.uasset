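; BP_Blitzball is the blitzball Blueprint, with a mesh that can be flagged for highlighting when focused.
; SetLastHit stores the player and pawn passed in as the ball's last hitter.
; OnBeginFocus and OnEndFocus toggle custom depth rendering and its stencil value on the mesh, marking it for a stencil-based effect.
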(fn `OnBeginFocus`
  (bind _blitzballmesh (`self.BlitzballMesh`))
  (`PrimitiveComponent.SetRenderCustomDepth` _blitzballmesh true)
  (`PrimitiveComponent.SetCustomDepthStencilValue` _blitzballmesh 255))

(fn `OnEndFocus`
  (bind _blitzballmesh (`self.BlitzballMesh`))
  (`PrimitiveComponent.SetRenderCustomDepth` _blitzballmesh false)
  (`PrimitiveComponent.SetCustomDepthStencilValue` _blitzballmesh 0))

(fn `SetLastHit`
  (params (Player :type "/Game/Blueprints/Online/BP_PlayerState Object Reference") (Pawn :type "/Game/Blueprints/Player/BP_Player Object Reference"))
  (`|ExecutionSequence`
    (:`then_0`
      (set `self.Player` Player))
    (:`then_1`
      (set `self.Pawn` Pawn))))

(fn `UserConstructionScript`)